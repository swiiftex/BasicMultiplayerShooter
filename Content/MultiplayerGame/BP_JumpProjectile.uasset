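; Multiplayer jump projectile that knocks first-person characters away from its impact point.
; On BeginPlay a server-to-multicast style event chain applies an impulse to the sphere, though the vector is zero as wired.
; On hit, it pushes characters overlapping SphereCollider by their scaled offset as a velocity change, via MCImpulse with authority or SRVImpulse on remote.
; It then expires almost immediately through a short lifespan.
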(event OnComponentHit(Sphere)
  (params (HitComponent :type Primitive%20Component%20Object%20Reference) (OtherActor :type Actor%20Object%20Reference) (OtherComp :type Primitive%20Component%20Object%20Reference) (NormalImpulse :type Vector :default "0, 0, 0") (Hit :type Hit%20Result%20Structure%20%28by%20ref%29))
  (for _array_element (Collision|GetOverlappingActors (Variables|Default|GetSphereCollider) "/Game/MultiplayerGame/BP_FirstPersonCharacter.BP_FirstPersonCharacter_C" :!class /Script/Engine.PrimitiveComponent)
    (bind _asbp_first_person_character (Utilities|Casting|CastToBP_FirstPersonCharacter _array_element))
    (Networking|SwitchHasAuthority
      (:Authority
        (Default|MCImpulse _asbp_first_person_character (* (- (Transformation|GetActorLocation _asbp_first_person_character) (Transformation|GetActorLocation self)) 0.3) true))
      (:Remote
        (Default|SRVImpulse _asbp_first_person_character (* (- (Transformation|GetActorLocation _asbp_first_person_character) (Transformation|GetActorLocation self)) 0.3) true))))
  (Actor|SetLifeSpan 0.1))

(event Custom|SRV%20Add%20impulse
  (CallFunction|MCAddIumpulse))

(event Custom|MC%20add%20iumpulse
  (Physics|AddImpulseatLocation (Variables|Default|GetSphere) (* "" (Variables|Default|GetInitial%20Speed)) "0, 0, 0" "None"))

(event EventBeginPlay
  (CallFunction|SRVAddImpulse))

(event Collision|EventActorBeginOverlap
  (params (OtherActor :type Actor%20Object%20Reference)))

(event EventTick
  (params (DeltaSeconds :type Float%20%28single-precision%29)))

(fn ConstructionScript)