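; BP_SpecPawn is the spectator pawn for the multiplayer shooter, letting a player request a respawn.
; Shortly after possession, it turns on the spectator view in HUD_Shooter for player 0.
; A left click fires RequestRespawn, which passes player 0's PlayerState to GS_Shooter's NotifyRespawnRequested and ignores its Controller input.
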(event Custom|Spec%20HUD
  (bind _ashud_shooter (Utilities|Casting|CastToHUD_Shooter (HUD|GetHUD (Game|GetPlayerController 0))))
  (Default|ToggleSpectatorHUD _ashud_shooter true))

(event Custom|Request%20Respawn
  (params (Controller :type Player%20Controller%20Object%20Reference))
  (bind _asgs_shooter (Utilities|Casting|CastToGS_Shooter (Game|GetGameState)))
  (Default|NotifyRespawnRequested _asgs_shooter (Game|GetPlayerState 0)))

(event EventBeginPlay)

(event EventPossessed
  (params (NewController :type Controller%20Object%20Reference))
  (Utilities|FlowControl|Delay 0.2)
  (CallFunction|SpecHUD))

(event Input|MouseEvents|LeftMouseButton
  (params (Key :type Key%20Structure :default "None"))
  (:Pressed
    (CallFunction|RequestRespawn (Game|GetPlayerController (Game|GetPlayerState 0)))))

(fn ConstructionScript)